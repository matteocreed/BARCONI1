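; Ground actor for the M9 weapon, built as a child that fills in the weapon-specific part of its parent.
; On BeginPlay it runs the parent logic, spawns an M9_A actor at the WeaponGround component's location and stores it as WeaponActor.
; It then copies that weapon's static mesh onto WeaponGround, so the ground mesh matches the spawned weapon.
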(event `self.ReceiveBeginPlay`
  (`parent.ReceiveBeginPlay`)
  (bind _returnvalue (`|SpawnActorFromClass` "/Game/MatteoCreed/Weapons/M9_A.M9_A_C" (`KismetMathLibrary.MakeTransform` (`SceneComponent.K2_GetComponentLocation` (`self.WeaponGround`))) "Undefined" "OverrideRootScale" null null))
  (bind _output_get (set `self.WeaponActor` _returnvalue))
  (`StaticMeshComponent.SetStaticMesh` (`self.WeaponGround`) (`/Game/MatteoCreed/Weapons/MasterWeapon_BP.WeaponStaticMesh` _output_get)))

(fn `UserConstructionScript`
  (`parent.UserConstructionScript`))