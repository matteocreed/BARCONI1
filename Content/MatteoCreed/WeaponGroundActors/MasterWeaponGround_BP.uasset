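; Base ground weapon pickup that hands its WeaponActor to a FirstPersonCharacter and destroys itself once collected.
; BeginPlay checks for characters already inside CollisionSphere, and sphere overlaps feed a DoOnce gate into the same CollectWeapon attempt.
; A failed collection resets the gate so pickup can be retried.
; TransferAmmo copies current and magazine ammo from a given weapon onto WeaponActor.
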(event `self.ReceiveBeginPlay`
  (bind _outactors (`GameplayStatics.GetAllActorsOfClass` "/Game/FirstPersonBP/Blueprints/FirstPersonCharacter.FirstPersonCharacter_C"))
  (for _array_element _outactors
    (if (`PrimitiveComponent.IsOverlappingActor` (`self.CollisionSphere`) _array_element)
      (bind _asfirst_person_character (cast `/Game/FirstPersonBP/Blueprints/FirstPersonCharacter` (stale `self.CollisionSphere.OnComponentBeginOverlap` OtherActor) :!label _label))
      (bind _success (`/Game/FirstPersonBP/Blueprints/FirstPersonCharacter.CollectWeapon` _asfirst_person_character (`self.WeaponActor`)))
      (if _success
        (`self.K2_DestroyActor`)
        (else
          (goto _label_2 :!via `Reset`))))))

(event `self.CollisionSphere.OnComponentBeginOverlap`
  (params (OverlappedComponent :type "PrimitiveComponent Object Reference") (OtherActor :type "Actor Object Reference") (OtherComp :type "PrimitiveComponent Object Reference") (OtherBodyIndex :type Integer) (bFromSweep :type Boolean) (SweepResult :type "HitResult Structure (by ref)"))
  (`/Engine/EditorBlueprintResources/StandardMacros.DoOnce` false :!label _label_2
    (:`Completed`
      (goto _label))))

(fn `TransferAmmo`
  (params (InWeapon :type "/Game/MatteoCreed/Weapons/MasterWeapon_BP Object Reference"))
  (bind _weaponactor (`self.WeaponActor`))
  (set `/Game/MatteoCreed/Weapons/MasterWeapon_BP.CurrentAmmo` (`/Game/MatteoCreed/Weapons/MasterWeapon_BP.CurrentAmmo` InWeapon) _weaponactor)
  (set `/Game/MatteoCreed/Weapons/MasterWeapon_BP.CurretMagAmmo` (`/Game/MatteoCreed/Weapons/MasterWeapon_BP.CurretMagAmmo` InWeapon) _weaponactor))

(fn `UserConstructionScript`)