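; Master weapon Blueprint that handles magazine and reserve ammo bookkeeping for a weapon.
; The construction script fills both counts to their maximums, and Fire spends one magazine round or prints an out-of-ammo message in Italian.
; CanReload checks for magazine space and remaining reserve.
; Reload tops up the magazine from reserve, but when reserve is insufficient it replaces the magazine count with the reserve instead of adding to it.
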(fn `CanReload`
  (returns (Success :type Boolean))
  (return (and (< (`self.CurretMagAmmo`) (`self.MaxMagAmmo`)) (> (`self.CurrentAmmo`) 0))))

(fn `Fire`
  (returns (CanFire :type Boolean))
  (if (> (`self.CurretMagAmmo`) 0)
    (`/Engine/EditorBlueprintResources/StandardMacros.DecrementInt` (`self.CurretMagAmmo`)
      (:`  `
        (return true)))
    (else
      (`KismetSystemLibrary.PrintString` "Hai finito i colpi")
      (return false))))

(fn `Reload`
  (returns (Success :type Boolean))
  (locals (Ammo_LOCAL :type Integer :default 0))
  (bind _output_get (set `local.Ammo_LOCAL` (- (`self.MaxMagAmmo`) (`self.CurretMagAmmo`))))
  (if (< _output_get (`self.CurrentAmmo`))
    (set `self.CurrentAmmo` (- (`self.CurrentAmmo`) (`local.Ammo_LOCAL`)))
    (set `self.CurretMagAmmo` (`self.MaxMagAmmo`))
    (else
      (set `self.CurretMagAmmo` (`self.CurrentAmmo`))
      (set `self.CurrentAmmo` 0)))
  (return true))

(fn `UserConstructionScript`
  (set `self.CurrentAmmo` (`self.MaxAmmo`))
  (set `self.CurretMagAmmo` (`self.MaxMagAmmo`)))