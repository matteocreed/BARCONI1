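; BP_BarconiTrack is an actor that lays out a straight spline, apparently as the base of a track.
; Its construction script adds local-space points along X, using NumberOfPoints as the spacing and TotalLenght divided by it, rounded, as the last index.
; Points are appended without clearing the spline's existing ones first.
; The event graph holds only disabled placeholder events, so the actor adds no runtime logic.
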(fn `UserConstructionScript`
  (for _index (range (+ (`KismetMathLibrary.Round` (/ (`self.TotalLenght`) (`KismetMathLibrary.Conv_IntToDouble` (`self.NumberOfPoints`)))) 1))
    (`SplineComponent.AddSplinePoint` (`self.Spline`) (`KismetMathLibrary.MakeVector` (`KismetMathLibrary.Conv_IntToDouble` (* (`self.NumberOfPoints`) _index))) "Local" true)))